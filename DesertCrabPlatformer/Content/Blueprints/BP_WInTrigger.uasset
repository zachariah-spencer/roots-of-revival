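; BP_WInTrigger is a level-completion trigger that fires when BP_PlantSpiderCharacter leaves its Box volume.
; The end-overlap event, rather than begin-overlap, calls LevelFinished, which a HasFinished flag limits to a single run.
; LevelFinished switches Wall collision to block everything, activates WinFX and adds the LevelComplete_WBP widget to the viewport.
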(event OnComponentEndOverlap(Box)
  (params (OverlappedComponent :type Primitive%20Component%20Object%20Reference) (OtherActor :type Actor%20Object%20Reference) (OtherComp :type Primitive%20Component%20Object%20Reference) (OtherBodyIndex :type Integer))
  (Utilities|Casting|CastToBP_PlantSpiderCharacter OtherActor)
  (CallFunction|LevelFinished))

(event EventBeginPlay)

(event Collision|EventActorBeginOverlap
  (params (OtherActor :type Actor%20Object%20Reference)))

(event EventTick
  (params (DeltaSeconds :type Float%20%28single-precision%29)))

(fn ConstructionScript)

(fn LevelFinished
  (if (not (Variables|Default|GetHasFinished))
    (Variables|Default|SetHasFinished true)
    (Collision|SetCollisionProfileName (Variables|Default|GetWall) "BlockAll" true :!class /Script/Engine.PrimitiveComponent)
    (Components|Activation|SetActive (Variables|Default|GetWinFX) true false)
    (bind _returnvalue (UserInterface|CreateWidget "/Game/UI/LevelComplete_WBP.LevelComplete_WBP_C" (Game|GetPlayerController 0)))
    (UserInterface|Viewport|AddtoViewport _returnvalue 0)))