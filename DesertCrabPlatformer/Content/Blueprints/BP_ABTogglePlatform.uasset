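; BP_ABTogglePlatform is a platform that flips each time the player's plant spider character jumps.
; It binds to that character's jump event, then activates a RotatingMovement pivoting around the Arrow's position, reversing the rotation rate each flip.
; After a short delay, Tick stops the rotation once pitch nears level, snaps pitch to zero and re-allows flipping.
; A looping timer for automatic flipping is left unconnected.
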(event OnComponentActivated(RotatingMovement)
  (params (Component :type Actor%20Component%20Object%20Reference) (bReset :type Boolean))
  (Variables|Default|SetCanActivate false)
  (Utilities|FlowControl|Delay 0.2)
  (Variables|Default|SetCanDeactivate true))

(event OnComponentDeactivated(RotatingMovement)
  (params (Component :type Actor%20Component%20Object%20Reference))
  (bind _platform (Variables|Default|GetPlatform))
  (bind _returnvalue (Transformation|GetWorldRotation _platform))
  (Transformation|SetWorldRotation _platform (Math|Rotator|MakeRotator (.roll _returnvalue) 0.0 (.yaw _returnvalue)) false true))

(event Custom|OnPlayerJumped
  (if (Variables|Default|GetCanActivate)
    (CallFunction|FlipPlatform)))

(event EventBeginPlay
  (Variables|/Script/Engine.RotatingMovementComponent|SetPivotTranslation (Variables|Default|GetRotatingMovement) (Variables|/Script/Engine.SceneComponent|GetRelativeLocation (Variables|Default|GetArrow)))
  (bind _asbp_plant_spider_character (Utilities|Casting|CastToBP_PlantSpiderCharacter (Game|Player|GetPlayerPawn 0)))
  (EventDispatchers|BindEventtoPlayerJumped _asbp_plant_spider_character (delegate Custom|OnPlayerJumped)))

(event EventTick
  (params (DeltaSeconds :type Float%20%28single-precision%29))
  (if (and (Components|Activation|IsActive (Variables|Default|GetRotatingMovement)) (Variables|Default|GetCanDeactivate))
    ;[1 1 1] Check when to deactivate rotation
    (if (Math|Float|NearlyEqual(Float) (.pitch (Transformation|GetWorldRotation (Variables|Default|GetPlatform))) 0.0 5.0)
      (Components|Activation|Deactivate (Variables|Default|GetRotatingMovement))
      (Variables|Default|SetCanActivate true))))

(fn ConstructionScript)

(fn FlipPlatform
  (bind _rotatingmovement (Variables|Default|GetRotatingMovement))
  (Variables|Default|SetCanDeactivate false)
  (Components|Activation|Activate _rotatingmovement false)
  (Variables|/Script/Engine.RotatingMovementComponent|SetRotationRate _rotatingmovement (* (Variables|/Script/Engine.RotatingMovementComponent|GetRotationRate _rotatingmovement) -1.0)))