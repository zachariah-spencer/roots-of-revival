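; BP_Hook is a swing anchor that registers itself as the plant spider character's NearbyHook while that character overlaps its swing-radius sphere.
; On BeginPlay it derives arc beginning, apex and end points from fixed world-axis offsets around itself, with the swing running along Y.
; Helper functions report arc progress from a Y position, using a hard-coded span and debug print, and whether the character overlaps the top-half box.
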(event OnComponentBeginOverlap(BeginSwingRadiusSphere)
  (params (OverlappedComponent :type Primitive%20Component%20Object%20Reference) (OtherActor :type Actor%20Object%20Reference) (OtherComp :type Primitive%20Component%20Object%20Reference) (OtherBodyIndex :type Integer) (bFromSweep :type Boolean) (SweepResult :type Hit%20Result%20Structure%20%28by%20ref%29))
  (bind _asbp_plant_spider_character (Utilities|Casting|CastToBP_PlantSpiderCharacter OtherActor))
  (Variables|/Game/ThirdPerson/Blueprints/BP_PlantSpiderCharacter.BP_PlantSpiderCharacter_C|SetNearbyHook _asbp_plant_spider_character self))

(event OnComponentEndOverlap(BeginSwingRadiusSphere)
  (params (OverlappedComponent :type Primitive%20Component%20Object%20Reference) (OtherActor :type Actor%20Object%20Reference) (OtherComp :type Primitive%20Component%20Object%20Reference) (OtherBodyIndex :type Integer))
  (bind _asbp_plant_spider_character (Utilities|Casting|CastToBP_PlantSpiderCharacter OtherActor))
  (Variables|/Game/ThirdPerson/Blueprints/BP_PlantSpiderCharacter.BP_PlantSpiderCharacter_C|SetNearbyHook _asbp_plant_spider_character 0))

(event EventBeginPlay
  (Variables|Default|SetArcApexPoint (+ (Transformation|GetActorLocation) "0.000000,0.000000,-500.000000"))
  (Variables|Default|SetArcBeginningPoint (+ (Transformation|GetActorLocation) "0.000000,-500.000000,0.000000"))
  (Variables|Default|SetArcEndPoint (+ (Transformation|GetActorLocation) "0.000000,500.000000,0.000000")))

(fn ConstructionScript)

(fn GetPercentageSwingArcCompleted
  (params (CurrentSwingingPosition :type Vector))
  (bind _returnvalue (+ (.y CurrentSwingingPosition) 1e+03))
  (bind _arcbeginningpoint (Variables|Default|GetArcBeginningPoint))
  (bind _arcendpoint (Variables|Default|GetArcEndPoint))
  (bind _returnvalue_2 (- _returnvalue (.y _arcbeginningpoint)))
  (bind _returnvalue_3 (- (.y _arcendpoint) (.y _arcbeginningpoint)))
  (bind _returnvalue_4 (- _returnvalue_2 _returnvalue_3))
  (bind _returnvalue_5 (/ _returnvalue_4 1e+03))
  (Development|PrintString (Utilities|String|ToString(Float) _returnvalue_5))
  (return _returnvalue_5))

(fn IsPlayerAboveHook
  (return (Utilities|Array|IsNotEmpty (Collision|GetOverlappingActors (Variables|Default|GetTopHalfCollisionBox) "/Game/ThirdPerson/Blueprints/BP_PlantSpiderCharacter.BP_PlantSpiderCharacter_C" :!class /Script/Engine.PrimitiveComponent))))