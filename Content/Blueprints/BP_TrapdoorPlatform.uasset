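; Trapdoor platform that drops away when something overlaps its trigger box, then returns to its starting transform.
; It briefly shows a telegraph plane, then physics and a downward impulse drop the cube while it ignores Pawn collision.
; After a delay, Tick lerps it toward the cached transform with a growing alpha until a timed snap finishes the reset.
; If the player pawn still overlaps the box, the drop repeats.
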(event OnComponentBeginOverlap(BoxCollision)
  (params (OverlappedComponent :type Primitive%20Component%20Object%20Reference) (OtherActor :type Actor%20Object%20Reference) (OtherComp :type Primitive%20Component%20Object%20Reference) (OtherBodyIndex :type Integer) (bFromSweep :type Boolean) (SweepResult :type Hit%20Result%20Structure%20%28by%20ref%29))
  (CallFunction|DropPlatform))

(event Custom|DropPlatform
  (if (not (Variables|Default|GetIsUsed))
    (Variables|Default|SetIsUsed true)
    (Rendering|SetVisibility (Variables|Default|GetTelegraphPlane) true false)
    (Utilities|FlowControl|Delay (Variables|Default|GetTelegraphDelayTime))
    (Rendering|SetVisibility (Variables|Default|GetTelegraphPlane) false false)
    (Physics|SetSimulatePhysics (Variables|Default|GetCube) true)
    (Physics|AddImpulse (Variables|Default|GetCube) "0.000000,0.000000,-2000.000000" "None" true)
    (Collision|SetCollisionResponsetoChannel (Variables|Default|GetCube) "ECC_Pawn" "ECR_Ignore")
    (Utilities|FlowControl|Delay (Variables|Default|GetUsedDelayTime))
    (Collision|SetCollisionResponsetoChannel (Variables|Default|GetCube) "ECC_Pawn" "ECR_Block")
    (Physics|SetSimulatePhysics (Variables|Default|GetCube) false)
    (Variables|Default|SetIsResetting true)
    (Utilities|FlowControl|Delay (Variables|Default|GetResetAnimationTime))
    (Variables|Default|SetIsResetting false)
    (Variables|Default|SetResettingAnimationAlpha 0.0)
    (Transformation|SetWorldLocationAndRotation (Variables|Default|GetCube) (Variables|Default|GetReadyLocation) (Variables|Default|GetReadyRotator) false true)
    (Variables|Default|SetIsUsed false)
    (if (Collision|IsOverlappingActor (Variables|Default|GetBoxCollision) (Game|Player|GetPlayerPawn 0) :!class /Script/Engine.PrimitiveComponent)
      (CallFunction|DropPlatform))))

(event EventBeginPlay
  (Variables|Default|SetReadyLocation (Transformation|GetWorldLocation (Variables|Default|GetCube)))
  (Variables|Default|SetReadyRotator (Transformation|GetWorldRotation (Variables|Default|GetCube))))

(event EventTick
  (params (DeltaSeconds :type Float%20%28single-precision%29))
  (bind _cube (Variables|Default|GetCube))
  (if (Variables|Default|GetIsResetting)
    (Transformation|SetWorldLocationAndRotation _cube (Math|Vector|Lerp(Vector) (Transformation|GetWorldLocation _cube) (Variables|Default|GetReadyLocation) (Variables|Default|GetResettingAnimationAlpha)) (Math|Rotator|Lerp(Rotator) (Transformation|GetWorldRotation _cube) (Variables|Default|GetReadyRotator) (Variables|Default|GetResettingAnimationAlpha) true) false false)
    (Variables|Default|SetResettingAnimationAlpha (+ (Variables|Default|GetResettingAnimationAlpha) 0.005))))

(fn ConstructionScript)